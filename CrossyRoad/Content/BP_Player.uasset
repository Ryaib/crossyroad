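; Player chicken that moves in discrete WASD steps and can be squashed, with car-squish and chicken sounds.
; Each key release adds movement input scaled by MaxSpeed and plays a random cluck.
; Tick consumes that input as a swept local offset, with no movement component involved.
; Death, not called within this Blueprint, runs once: it zeroes MaxSpeed, flattens the mesh, plays death sounds and sets IsDead, which silences clucks.
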(event EventBeginPlay)

(event Collision|EventActorBeginOverlap
  (params (OtherActor :type Actor%20Object%20Reference)))

(event EventTick
  (params (DeltaSeconds :type Float%20%28single-precision%29))
  (bind _returnvalue (Class|Pawn|ConsumeMovementInputVector))
  (Transformation|AddActorLocalOffset _returnvalue true false))

(event Input|KeyboardEvents|D
  (params (Key :type Key%20Structure))
  (:Released
    (Pawn|Input|AddMovementInput (Transformation|GetActorRightVector) (Variables|Default|GetMaxSpeed) false)
    (CallFunction|RandomMoveSound)))

(event Input|KeyboardEvents|W
  (params (Key :type Key%20Structure))
  (:Released
    (Pawn|Input|AddMovementInput (Transformation|GetActorForwardVector) (Variables|Default|GetMaxSpeed) false)
    (CallFunction|RandomMoveSound)))

(event Input|KeyboardEvents|A
  (params (Key :type Key%20Structure))
  (:Released
    (Pawn|Input|AddMovementInput (* (Transformation|GetActorRightVector) "-1.000000,-1.000000,-1.000000") (Variables|Default|GetMaxSpeed) false)
    (CallFunction|RandomMoveSound)))

(event Input|KeyboardEvents|S
  (params (Key :type Key%20Structure))
  (:Released
    (Pawn|Input|AddMovementInput (* (Transformation|GetActorForwardVector) "-1.000000,-1.000000,-1.000000") (Variables|Default|GetMaxSpeed) false)
    (CallFunction|RandomMoveSound)))

(fn ConstructionScript)

(fn Death
  (if (not (Variables|Default|GetisDead))
    (Variables|Default|SetMaxSpeed 0.0)
    (Class|SceneComponent|AddLocalTransform (Variables|Default|GetStaticMesh) (Math|Transform|MakeTransform "0, 0, 0" "0, 0, 0" "1,0.100000,1") false false)
    (Audio|PlaySound2D "/Game/carsquish3.carsquish3" 1.0 1.0 0.0 0 0)
    (Audio|PlaySound2D (Utilities|Select :Index (Math|Random|RandomIntegerinRange 0 1) :Option%200 "/Game/chickendeath.chickendeath" :Option%201 "/Game/chickendeath2.chickendeath2") 1.0 1.0 0.0 0 0)
    (Variables|Default|SetisDead true)))

(fn RandomMoveSound
  (if (not (Variables|Default|GetisDead))
    (Audio|PlaySound2D (Utilities|Select :Index (Math|Random|RandomIntegerinRange 0 11) :Option%200 "/Game/Clucks/buck1.buck1" :Option%201 "/Game/Clucks/buck2.buck2" :Option%202 "/Game/Clucks/buck3.buck3" :Option%203 "/Game/Clucks/buck4.buck4" :Option%204 "/Game/Clucks/buck5.buck5" :Option%205 "/Game/Clucks/buck6.buck6" :Option%206 "/Game/Clucks/buck7.buck7" :Option%207 "/Game/Clucks/buck8.buck8" :Option%208 "/Game/Clucks/buck9.buck9" :Option%209 "/Game/Clucks/buck10.buck10" :Option%2010 "/Game/Clucks/buck11.buck11" :Option%2011 "/Game/Clucks/buck12.buck12") 1.0 1.0 0.0 0 0)))