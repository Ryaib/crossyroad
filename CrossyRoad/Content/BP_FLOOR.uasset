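; BP_FLOOR is a self-replenishing road segment that fills three roads with moving-traffic obstacles for the player.
; BeginPlay spawns six cars and trucks at lane spawn points; end-of-lane triggers teleport each stored vehicle back and randomize the overlapping vehicle's speed.
; When BP_Player enters TriggerZone, FloorSpawner adds another floor.
; When BP_Player enters DestroyZone, the segment destroys itself and its vehicles.
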(event OnComponentBeginOverlap(Road1_SouthEnd)
  (params (OverlappedComponent :type Primitive%20Component%20Object%20Reference) (OtherActor :type Actor%20Object%20Reference) (OtherComp :type Primitive%20Component%20Object%20Reference) (OtherBodyIndex :type Integer) (bFromSweep :type Boolean) (SweepResult :type Hit%20Result%20Structure%20%28by%20ref%29))
  (bind _asred_car (Utilities|Casting|CastToRED_CAR OtherActor))
  (Transformation|Teleport (Variables|Default|GetSpawnedCar) (Transformation|GetWorldLocation (Variables|Default|GetSpawnPoint1)) "0, 0, 0")
  (Default|RandomizeSpeed _asred_car))

(event OnComponentBeginOverlap(TriggerZone)
  (params (OverlappedComponent :type Primitive%20Component%20Object%20Reference) (OtherActor :type Actor%20Object%20Reference) (OtherComp :type Primitive%20Component%20Object%20Reference) (OtherBodyIndex :type Integer) (bFromSweep :type Boolean) (SweepResult :type Hit%20Result%20Structure%20%28by%20ref%29))
  (Utilities|Casting|CastToBP_Player OtherActor)
  (Default|SpawnFlooratPoint (Variables|Default|GetFloorSpawner)))

(event OnComponentBeginOverlap(DestroyZone)
  (params (OverlappedComponent :type Primitive%20Component%20Object%20Reference) (OtherActor :type Actor%20Object%20Reference) (OtherComp :type Primitive%20Component%20Object%20Reference) (OtherBodyIndex :type Integer) (bFromSweep :type Boolean) (SweepResult :type Hit%20Result%20Structure%20%28by%20ref%29))
  (Utilities|Casting|CastToBP_Player OtherActor)
  (Actor|DestroyActor)
  (Actor|DestroyActor (Variables|Default|GetSpawnedCar))
  (Actor|DestroyActor (Variables|Default|GetBlueCar))
  (Actor|DestroyActor (Variables|Default|GetTruck1))
  (Actor|DestroyActor (Variables|Default|GetCar4))
  (Actor|DestroyActor (Variables|Default|GetCar5))
  (Actor|DestroyActor (Variables|Default|GetTruck6)))

(event OnComponentBeginOverlap(Road1_NorthEnd)
  (params (OverlappedComponent :type Primitive%20Component%20Object%20Reference) (OtherActor :type Actor%20Object%20Reference) (OtherComp :type Primitive%20Component%20Object%20Reference) (OtherBodyIndex :type Integer) (bFromSweep :type Boolean) (SweepResult :type Hit%20Result%20Structure%20%28by%20ref%29))
  (bind _asblue_car_bp (Utilities|Casting|CastToBLUE_CAR_BP OtherActor))
  (Transformation|Teleport (Variables|Default|GetBlueCar) (Transformation|GetWorldLocation (Variables|Default|GetSpawnPoint2)) "0, 0, 0")
  (Default|RandomizeSpeed _asblue_car_bp))

(event OnComponentBeginOverlap(Road2_SouthEnd)
  (params (OverlappedComponent :type Primitive%20Component%20Object%20Reference) (OtherActor :type Actor%20Object%20Reference) (OtherComp :type Primitive%20Component%20Object%20Reference) (OtherBodyIndex :type Integer) (bFromSweep :type Boolean) (SweepResult :type Hit%20Result%20Structure%20%28by%20ref%29))
  (bind _asbp_truck (Utilities|Casting|CastToBP_TRUCK OtherActor))
  (Transformation|Teleport (Variables|Default|GetTruck1) (Transformation|GetWorldLocation (Variables|Default|GetSpawnPoint3)) "0, 0, 0")
  (Default|RandomizeSpeed _asbp_truck))

(event OnComponentBeginOverlap(Road2_NorthEnd)
  (params (OverlappedComponent :type Primitive%20Component%20Object%20Reference) (OtherActor :type Actor%20Object%20Reference) (OtherComp :type Primitive%20Component%20Object%20Reference) (OtherBodyIndex :type Integer) (bFromSweep :type Boolean) (SweepResult :type Hit%20Result%20Structure%20%28by%20ref%29))
  (bind _asred_car (Utilities|Casting|CastToRED_CAR OtherActor))
  (Transformation|Teleport (Variables|Default|GetCar4) (Transformation|GetWorldLocation (Variables|Default|GetSpawnPoint4)) "0,-180.000000, 0")
  (Default|RandomizeSpeed _asred_car))

(event OnComponentBeginOverlap(Road3_South1)
  (params (OverlappedComponent :type Primitive%20Component%20Object%20Reference) (OtherActor :type Actor%20Object%20Reference) (OtherComp :type Primitive%20Component%20Object%20Reference) (OtherBodyIndex :type Integer) (bFromSweep :type Boolean) (SweepResult :type Hit%20Result%20Structure%20%28by%20ref%29))
  (bind _asblue_car_bp (Utilities|Casting|CastToBLUE_CAR_BP OtherActor))
  (Transformation|Teleport (Variables|Default|GetCar5) (Transformation|GetWorldLocation (Variables|Default|GetRoad3%20Spawn1)) "0,180.000000, 0")
  (Default|RandomizeSpeed _asblue_car_bp))

(event OnComponentBeginOverlap(Road3_South2)
  (params (OverlappedComponent :type Primitive%20Component%20Object%20Reference) (OtherActor :type Actor%20Object%20Reference) (OtherComp :type Primitive%20Component%20Object%20Reference) (OtherBodyIndex :type Integer) (bFromSweep :type Boolean) (SweepResult :type Hit%20Result%20Structure%20%28by%20ref%29))
  (bind _asbp_truck (Utilities|Casting|CastToBP_TRUCK OtherActor))
  (Transformation|Teleport (Variables|Default|GetTruck6) (Transformation|GetWorldLocation (Variables|Default|GetTruck2Spawn)) "0, 0, 0")
  (Default|RandomizeSpeed _asbp_truck))

(event EventBeginPlay
  (Utilities|FlowControl|Sequence
    (:then_0
      (bind _returnvalue (Game|SpawnActorfromClass "/Game/RED_CAR.RED_CAR_C" (Math|Transform|MakeTransform (Transformation|GetWorldLocation (Variables|Default|GetSpawnPoint1)) "0, 0, 0" "1,1,1") "Undefined" 0 0))
      (Variables|Default|SetSpawnedCar _returnvalue))
    (:then_1
      (bind _returnvalue_2 (Game|SpawnActorfromClass "/Game/BLUE_CAR_BP.BLUE_CAR_BP_C" (Math|Transform|MakeTransform (Transformation|GetWorldLocation (Variables|Default|GetSpawnPoint2)) "0, 0, 0" "1,1,1") "Undefined" 0 0))
      (Variables|Default|SetBlueCar _returnvalue_2))
    (:then_2
      (bind _returnvalue_3 (Game|SpawnActorfromClass "/Game/BP_TRUCK.BP_TRUCK_C" (Math|Transform|MakeTransform (Transformation|GetWorldLocation (Variables|Default|GetSpawnPoint3)) "0, 0, 0" "1,1,1") "Undefined" 0 0))
      (Variables|Default|SetTruck1 _returnvalue_3))
    (:then_3
      (bind _returnvalue_4 (Game|SpawnActorfromClass "/Game/RED_CAR.RED_CAR_C" (Math|Transform|MakeTransform (Transformation|GetWorldLocation (Variables|Default|GetSpawnPoint4)) "0.000000,-180.000000, 0" "1,1,1") "Undefined" 0 0))
      (Variables|Default|SetCar4 _returnvalue_4))
    (:then_4
      (bind _returnvalue_5 (Game|SpawnActorfromClass "/Game/BLUE_CAR_BP.BLUE_CAR_BP_C" (Math|Transform|MakeTransform (Transformation|GetWorldLocation (Variables|Default|GetRoad3%20Spawn1)) "0,180.000000, 0" "1,1,1") "Undefined" 0 0))
      (Variables|Default|SetCar5 _returnvalue_5))
    (:then_5
      (bind _returnvalue_6 (Game|SpawnActorfromClass "/Game/BP_TRUCK.BP_TRUCK_C" (Math|Transform|MakeTransform (Transformation|GetWorldLocation (Variables|Default|GetTruck2Spawn)) "0, 0, 0" "1,1,1") "Undefined" 0 0))
      (Variables|Default|SetTruck6 _returnvalue_6))))

(event Collision|EventActorBeginOverlap
  (params (OtherActor :type Actor%20Object%20Reference)))

(event EventTick
  (params (DeltaSeconds :type Float%20%28single-precision%29)))

(fn ConstructionScript)