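; BP_TRUCK is a moving truck hazard that kills the player on contact.
; On BeginPlay it picks a random MaxSpeed, then each Tick moves itself along its local Y axis with a swept, frame-rate-independent offset.
; When its StaticMesh begins overlapping a BP_Player, it calls that player's Death.
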(event OnComponentBeginOverlap(StaticMesh)
  (params (OverlappedComponent :type Primitive%20Component%20Object%20Reference) (OtherActor :type Actor%20Object%20Reference) (OtherComp :type Primitive%20Component%20Object%20Reference) (OtherBodyIndex :type Integer) (bFromSweep :type Boolean) (SweepResult :type Hit%20Result%20Structure%20%28by%20ref%29))
  (bind _asbp_player (Utilities|Casting|CastToBP_Player OtherActor))
  (Default|Death _asbp_player))

(event EventBeginPlay
  (CallFunction|RandomizeSpeed))

(event Collision|EventActorBeginOverlap
  (params (OtherActor :type Actor%20Object%20Reference)))

(event EventTick
  (params (DeltaSeconds :type Float%20%28single-precision%29))
  (Transformation|AddActorLocalOffset (Math|Vector|MakeVector 0.0 (* DeltaSeconds (Variables|Default|GetMaxSpeed)) 0.0) true false))

(fn ConstructionScript)

(fn RandomizeSpeed
  (Variables|Default|SetMaxSpeed (Math|Random|RandomFloatinRange 1e+02 4e+02)))